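; BP_OfficeGuy is an interactable office NPC that the top-down player character can talk to.
; Its trigger overlap registers it as the player's current NPC and shows a prompt widget, clearing both when the player leaves.
; While interaction is possible, Tick rotates the widget toward the controller's view target.
; TrytoTalk disables player controller input, opens a dialogue window through the player character and fills it from the first line.
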(event OnComponentBeginOverlap(Trigger)
  (params (OverlappedComponent :type Primitive%20Component%20Object%20Reference) (OtherActor :type Actor%20Object%20Reference) (OtherComp :type Primitive%20Component%20Object%20Reference) (OtherBodyIndex :type Integer) (bFromSweep :type Boolean) (SweepResult :type Hit%20Result%20Structure%20%28by%20ref%29))
  ;[0.15 0.15 0.15 0.5] Overlapping
  (Utilities|Casting|CastToBP_TopDownCharacter OtherActor)
  (Variables|/Game/1_Blueprints/BP_TopDownCharacter.BP_TopDownCharacter_C|SetNPC (Variables|Default|GetPlayerRef) self)
  (Variables|Default|SetCanInteract true)
  (Development|SetHiddeninGame (Variables|Default|GetWidget) false false))

(event OnComponentEndOverlap(Trigger)
  (params (OverlappedComponent :type Primitive%20Component%20Object%20Reference) (OtherActor :type Actor%20Object%20Reference) (OtherComp :type Primitive%20Component%20Object%20Reference) (OtherBodyIndex :type Integer))
  ;[0.15 0.15 0.15 0.5] Overlapping
  (Utilities|Casting|CastToBP_TopDownCharacter OtherActor)
  (Variables|/Game/1_Blueprints/BP_TopDownCharacter.BP_TopDownCharacter_C|SetNPC (Variables|Default|GetPlayerRef) 0)
  (Variables|Default|SetCanInteract false)
  (Development|SetHiddeninGame (Variables|Default|GetWidget) true false))

(event EventBeginPlay
  (bind _asbp_top_down_character (Utilities|Casting|CastToBP_TopDownCharacter (Game|Player|GetPlayerPawn 0)))
  (Variables|Default|SetPlayerRef _asbp_top_down_character)
  (Development|SetHiddeninGame (Variables|Default|GetWidget) true false))

(event EventTick
  (params (DeltaSeconds :type Float%20%28single-precision%29))
  (bind _widget (Variables|Default|GetWidget))
  (if (Variables|Default|GetCanInteract)
    (Transformation|SetWorldRotation _widget (Math|Rotator|FindLookatRotation (Transformation|GetWorldLocation _widget) (Transformation|GetActorLocation (Pawn|GetViewTarget (Variables|/Game/1_Blueprints/BP_TopDownCharacter.BP_TopDownCharacter_C|GetControllerRef (Variables|Default|GetPlayerRef))))) false false)))

(event EventTrytoTalk
  (bind _playerref (Variables|Default|GetPlayerRef))
  (bind _controllerref (Variables|/Game/1_Blueprints/BP_TopDownCharacter.BP_TopDownCharacter_C|GetControllerRef _playerref))
  (Input|DisableInput _controllerref _controllerref)
  (bind _dialoguewindow (Default|BeginDialogue (Variables|Default|GetPlayerRef)))
  (bind _output_get (Variables|Default|SetDialogueWindow _dialoguewindow))
  (Variables|Default|SetCurrentLine 0)
  (CallFunction|FillText _output_get))

(fn ConstructionScript
  (|CallParentFunction))