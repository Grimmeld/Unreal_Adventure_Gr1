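; BP_NPCBase is a base NPC Blueprint that holds shared dialogue state and helpers for conversations.
; FillText pushes the name, portrait and text of the dialogue entry at CurrentLine into a dialogue widget.
; CheckIndex reports when CurrentLine has passed the last entry, and EndDiscussion resets the line and clears the window reference.
; TryToTalk is an empty event, and nothing here advances the line or creates the widget.
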(event Custom|FillText
  (params (DialogueWidget :type WBP%20Dialogue%20Object%20Reference) (Dialogues :type Array%20of%20F%20Dialogues%20Structures))
  (bind _currentline (Variables|Default|GetCurrentLine))
  (bind _output (Utilities|Array|Get(acopy) Dialogues _currentline))
  (bind (_namenpc _imagenpc _lines) (Utilities|Struct|BreakFDialogues _output))
  (Default|SetName DialogueWidget _namenpc)
  (Default|SetIcon DialogueWidget _imagenpc)
  (Default|SetDialogue DialogueWidget _lines))

(event Custom|EndDiscussion
  (Variables|Default|SetCurrentLine 0)
  (Variables|Default|SetDialogueWindow 0))

(event Custom|TryToTalk)

(event EventBeginPlay)

(event Collision|EventActorBeginOverlap
  (params (OtherActor :type Actor%20Object%20Reference)))

(event EventTick
  (params (DeltaSeconds :type Float%20%28single-precision%29)))

(fn ConstructionScript)

(fn CheckIndex
  (return (>= (Variables|Default|GetCurrentLine) (Utilities|Array|Length (Variables|Default|GetDialogues)))))