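; BP_ItemBase is a base world item that registers itself with the top-down player character as the current interactable.
; The construction script applies mesh and trigger radius from its Data, which GetItemData exposes.
; Trigger overlaps call SetItem on the player to set or end interaction.
; OnInteraction only clears CanInteract; the interact widget stays hidden because its visibility toggle is disconnected.
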(event OnComponentBeginOverlap(TriggerCollision)
  (params (OverlappedComponent :type Primitive%20Component%20Object%20Reference) (OtherActor :type Actor%20Object%20Reference) (OtherComp :type Primitive%20Component%20Object%20Reference) (OtherBodyIndex :type Integer) (bFromSweep :type Boolean) (SweepResult :type Hit%20Result%20Structure%20%28by%20ref%29))
  ;[0.15 0.15 0.15 0.5] Action Interaction
  (Utilities|Casting|CastToBP_TopDownCharacter OtherActor)
  (CallFunction|OnInteraction true)
  (Default|SetItem (Variables|Reference|GetPlayerRef) self true))

(event OnComponentEndOverlap(TriggerCollision)
  (params (OverlappedComponent :type Primitive%20Component%20Object%20Reference) (OtherActor :type Actor%20Object%20Reference) (OtherComp :type Primitive%20Component%20Object%20Reference) (OtherBodyIndex :type Integer))
  ;[0.15 0.15 0.15 0.5] Action Interaction
  (Utilities|Casting|CastToBP_TopDownCharacter OtherActor)
  (CallFunction|OnInteraction false)
  (Default|SetItem (Variables|Reference|GetPlayerRef) 0 false))

(event Custom|PrepareItem
  (bind _data (Variables|Default|GetData))
  (Utilities|IsValid _data
    (:Is%20Valid
      (Components|StaticMesh|SetStaticMesh (Variables|Default|GetMesh) (Variables|/Game/1_Blueprints/Items/Datas/PDA_Items.PDA_Items_C|GetMesh _data))
      (Components|Sphere|SetSphereRadius (Variables|Default|GetTriggerCollision) (Variables|/Game/1_Blueprints/Items/Datas/PDA_Items.PDA_Items_C|GetCollisionRadius _data) true))))

(event Custom|OnInteraction
  (params (IsInteracting :type Boolean))
  ;[0.15 0.15 0.15 0.5] Action Interaction
  (Variables|Default|SetCanInteract false))

(event EventBeginPlay
  (bind _asbp_top_down_character (Utilities|Casting|CastToBP_TopDownCharacter (Game|Player|GetPlayerPawn 0)))
  (Variables|Reference|SetPlayerRef _asbp_top_down_character)
  (Development|SetHiddeninGame (Variables|Default|GetWidgetInteract) true false))

(fn ConstructionScript
  (CallFunction|PrepareItem))

(fn GetItemData
  (return (Variables|Default|GetData)))