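; BP_Vista is a trigger that switches the player's view to a vista camera.
; When a BP_TopDownCharacter begins overlapping CollisionTrigger, it blends that character's controller view target to CameraVista using configurable blend time, function and exponent.
; The switch is one-way, as nothing here restores the view when the overlap ends.
; BeginPlay prints a warning naming the actor if CameraVista is not valid.
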(event OnComponentBeginOverlap(CollisionTrigger)
  (params (OverlappedComponent :type Primitive%20Component%20Object%20Reference) (OtherActor :type Actor%20Object%20Reference) (OtherComp :type Primitive%20Component%20Object%20Reference) (OtherBodyIndex :type Integer) (bFromSweep :type Boolean) (SweepResult :type Hit%20Result%20Structure%20%28by%20ref%29))
  (bind _asbp_top_down_character (Utilities|Casting|CastToBP_TopDownCharacter OtherActor))
  (if (Utilities|IsValid (Variables|Default|GetCameraVista))
    (Game|Player|SetViewTargetwithBlend (Variables|/Game/1_Blueprints/BP_TopDownCharacter.BP_TopDownCharacter_C|GetControllerRef _asbp_top_down_character) (Variables|Default|GetCameraVista) (Variables|Blend|GetBlend%20Time) (Variables|Blend|GetBlend%20Func) (Variables|Blend|GetBlend%20Exp) false)))

(event EventBeginPlay
  ;[0.15 0.15 0.15 0.5] Camera not valid
  (Utilities|IsValid (Variables|Default|GetCameraVista)
    (:Is%20Not%20Valid
      (Development|PrintString (Utilities|String|Append "Camera not found for " (Utilities|GetObjectName self))))))

(fn ConstructionScript)