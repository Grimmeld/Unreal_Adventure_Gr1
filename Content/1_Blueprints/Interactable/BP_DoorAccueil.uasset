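; Double reception door that is locked from one side until the player character reaches its back trigger.
; Entering that trigger enables interaction through InteractionDoor and clears the lock, which is not restored on exit, when only the widget is disabled.
; OpenDoor logs a locked message to the player's HUD while locked.
; Otherwise it hides the widget, starts two timelines that rotate the door pivots in yaw, and marks the door unlocked.
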(event OnComponentBeginOverlap(TriggerBack)
  (params (OverlappedComponent :type Primitive%20Component%20Object%20Reference) (OtherActor :type Actor%20Object%20Reference) (OtherComp :type Primitive%20Component%20Object%20Reference) (OtherBodyIndex :type Integer) (bFromSweep :type Boolean) (SweepResult :type Hit%20Result%20Structure%20%28by%20ref%29))
  (bind _asbp_top_down_character (Utilities|Casting|CastToBP_TopDownCharacter OtherActor))
  (CallFunction|InteractionDoor _asbp_top_down_character true false false)
  (Variables|Default|SetisLockedFromBack false))

(event OnComponentEndOverlap(TriggerBack)
  (params (OverlappedComponent :type Primitive%20Component%20Object%20Reference) (OtherActor :type Actor%20Object%20Reference) (OtherComp :type Primitive%20Component%20Object%20Reference) (OtherBodyIndex :type Integer))
  (bind _asbp_top_down_character (Utilities|Casting|CastToBP_TopDownCharacter OtherActor))
  (CallFunction|InteractionDoor _asbp_top_down_character false true false))

(event EventBeginPlay
  (|CallParentFunction))

(event Collision|EventActorBeginOverlap
  (params (OtherActor :type Actor%20Object%20Reference))
  (|CallParentFunction OtherActor) ; This node is disabled and will not be called.\nDrag off pins to build functionality.
)

(event EventTick
  (params (DeltaSeconds :type Float%20%28single-precision%29))
  (|CallParentFunction DeltaSeconds) ; This node is disabled and will not be called.\nDrag off pins to build functionality.
)

(event EventOpenDoor
  (if (Variables|Default|GetisLockedFromBack)
    (Default|AddMessageLog (Variables|/Game/1_Blueprints/BP_TopDownCharacter.BP_TopDownCharacter_C|GetHUDRef (Variables|Default|GetPlayerRef)) (Variables|Default|GetDoorLockedLog))
    (else
      (Variables|Default|SethasInteracted true)
      (Development|SetHiddeninGame (Variables|Default|Get%20Widget) true false)
      (Utilities|FlowControl|Sequence
        (:then_0
          (bind _rotationpivot (Timeline|OuverturePorte1 Play)
            (:Update
              (Transformation|SetRelativeRotation (Variables|Default|GetPointDoor1) (Math|Rotator|MakeRotator 0.0 0.0 _rotationpivot) false false))))
        (:then_1
          (bind _rotationpivot_2 (Timeline|OuverturePorte2 Play)
            (:Update
              (Transformation|SetRelativeRotation (Variables|Default|GetPointDoor2) (Math|Rotator|MakeRotator 0.0 0.0 _rotationpivot_2) false false))))
        (:then_2
          (Variables|Default|SetisUnlocked true))))))

(fn ConstructionScript
  (|CallParentFunction))