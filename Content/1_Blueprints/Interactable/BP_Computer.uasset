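; Interactable computer that starts the player's computer game and unlocks a PC code clue.
; Its Trigger overlap registers it as the top-down character's current interactable and toggles the interaction prompt, clearing both on exit.
; On use it plays a keyboard sound and calls BeginComputerGame on the cached player.
; The first use also plays the HUD clue-noted animation and reveals the clue in the notebook (Calepin), guarded by the FirstTime flag.
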(event OnComponentBeginOverlap(Trigger)
  (params (OverlappedComponent :type Primitive%20Component%20Object%20Reference) (OtherActor :type Actor%20Object%20Reference) (OtherComp :type Primitive%20Component%20Object%20Reference) (OtherBodyIndex :type Integer) (bFromSweep :type Boolean) (SweepResult :type Hit%20Result%20Structure%20%28by%20ref%29))
  (bind _asbp_top_down_character (Utilities|Casting|CastToBP_TopDownCharacter OtherActor))
  (Default|SetInteractable _asbp_top_down_character self)
  (Default|DisplayWidgetInteraction (Variables|Default|GetPlayerRef) true))

(event OnComponentEndOverlap(Trigger)
  (params (OverlappedComponent :type Primitive%20Component%20Object%20Reference) (OtherActor :type Actor%20Object%20Reference) (OtherComp :type Primitive%20Component%20Object%20Reference) (OtherBodyIndex :type Integer))
  (bind _asbp_top_down_character (Utilities|Casting|CastToBP_TopDownCharacter OtherActor))
  (Default|SetInteractable _asbp_top_down_character)
  (Default|DisplayWidgetInteraction (Variables|Default|GetPlayerRef) false))

(event EventBeginPlay
  (|CallParentFunction)
  (bind _asbp_top_down_character (Utilities|Casting|CastToBP_TopDownCharacter (Game|Player|GetPlayerPawn 0)))
  (Variables|Default|SetPlayerRef _asbp_top_down_character))

(event Collision|EventActorBeginOverlap
  (params (OtherActor :type Actor%20Object%20Reference))
  (|CallParentFunction OtherActor) ; This node is disabled and will not be called.\nDrag off pins to build functionality.
)

(event EventTick
  (params (DeltaSeconds :type Float%20%28single-precision%29))
  (|CallParentFunction DeltaSeconds) ; This node is disabled and will not be called.\nDrag off pins to build functionality.
)

(event EventUseInteractable
  (bind _playerref (Variables|Default|GetPlayerRef))
  (Audio|PlaySound2D "/Game/8_Sound/SFX/KeyboardTouch.KeyboardTouch" 1.0 1.0 0.0 0 0)
  (Default|BeginComputerGame _playerref)
  (if (not (Variables|Default|GetFirstTime?))
    (Default|CluesNotedAnim (Variables|/Game/1_Blueprints/BP_TopDownCharacter.BP_TopDownCharacter_C|GetHUDRef _playerref))
    (Default|RevealClues (Variables|/Game/1_Blueprints/BP_TopDownCharacter.BP_TopDownCharacter_C|GetCalepinRef _playerref) "Clues4_PCcode")
    (Variables|Default|SetFirstTime? true)))

(fn ConstructionScript
  (|CallParentFunction))