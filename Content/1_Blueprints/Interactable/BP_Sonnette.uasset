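; BP_Sonnette is an interactable save point that stores game progress when the player uses it.
; Its trigger overlap registers it as the character's interactable and toggles the interact prompt widget.
; On use, unless a save is already flagged, it sets that flag and sends player, item and door save messages to the Game Instance.
; It then shows the saving widget and adds an audio component.
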(event OnComponentBeginOverlap(Trigger)
  (params (OverlappedComponent :type Primitive%20Component%20Object%20Reference) (OtherActor :type Actor%20Object%20Reference) (OtherComp :type Primitive%20Component%20Object%20Reference) (OtherBodyIndex :type Integer) (bFromSweep :type Boolean) (SweepResult :type Hit%20Result%20Structure%20%28by%20ref%29))
  (bind _playerref (Variables|Reference|GetPlayerRef))
  (bind _asbp_top_down_character (Utilities|Casting|CastToBP_TopDownCharacter OtherActor))
  (Default|SetInteractable _asbp_top_down_character self)
  (Variables|/Game/1_Blueprints/BP_TopDownCharacter.BP_TopDownCharacter_C|SetCanInteractChara _playerref true)
  (Development|SetHiddeninGame (Variables|/Game/1_Blueprints/BP_TopDownCharacter.BP_TopDownCharacter_C|GetWidget_Interact _playerref) false false))

(event OnComponentEndOverlap(Trigger)
  (params (OverlappedComponent :type Primitive%20Component%20Object%20Reference) (OtherActor :type Actor%20Object%20Reference) (OtherComp :type Primitive%20Component%20Object%20Reference) (OtherBodyIndex :type Integer))
  (bind _playerref (Variables|Reference|GetPlayerRef))
  (bind _asbp_top_down_character (Utilities|Casting|CastToBP_TopDownCharacter OtherActor))
  (Default|SetInteractable _asbp_top_down_character)
  (Variables|/Game/1_Blueprints/BP_TopDownCharacter.BP_TopDownCharacter_C|SetCanInteractChara _playerref false)
  (Development|SetHiddeninGame (Variables|/Game/1_Blueprints/BP_TopDownCharacter.BP_TopDownCharacter_C|GetWidget_Interact _playerref) true false))

(event EventBeginPlay
  (bind _asbp_top_down_character (Utilities|Casting|CastToBP_TopDownCharacter (Game|Player|GetPlayerPawn 0)))
  (Variables|Reference|SetPlayerRef _asbp_top_down_character))

(event EventUseInteractable
  (bind _returnvalue (Game|GetGameInstance))
  (bind _playerref (Variables|Reference|GetPlayerRef))
  (bind _playerref_2 (Variables|Reference|GetPlayerRef))
  (if (not (Variables|/Game/1_Blueprints/BP_TopDownCharacter.BP_TopDownCharacter_C|GetisSaving _playerref_2))
    (Variables|/Game/1_Blueprints/BP_TopDownCharacter.BP_TopDownCharacter_C|SetisSaving _playerref_2 true)
    (bind _playersave (Default|GetPlayerSave _playerref))
    (Class|BISaveGame|SavePlayer(Message) _returnvalue _playersave)
    (Class|BISaveGame|SaveItems(Message) _returnvalue)
    (Class|BISaveGame|SaveDoors(Message) _returnvalue)
    (Default|ShowSavingWidget _playerref)
    (AddComponent|AddAudioComponent false)))

(fn ConstructionScript)