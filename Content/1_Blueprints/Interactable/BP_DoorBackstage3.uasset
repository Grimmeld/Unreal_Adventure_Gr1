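; BP_DoorBackstage3 is an interactable backstage double door that swings open on two pivot components.
; OpenDoor flags the interaction, hides the prompt widget, plays a separate timeline per pivot to drive its yaw, and marks the door unlocked.
; On BeginPlay, a door already flagged as unlocked snaps straight to its open rotation, with the two pivots turned in opposite directions.
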(event EventBeginPlay
  (|CallParentFunction)
  (if (Variables|Default|GetisUnlocked)
    (Transformation|SetRelativeRotation (Variables|Default|GetPointDoor1) (Math|Rotator|MakeRotator 0.0 0.0 1.1e+02) false false)
    (Transformation|SetRelativeRotation (Variables|Default|GetPointDoor2) (Math|Rotator|MakeRotator 0.0 0.0 -1.1e+02) false false)))

(event Collision|EventActorBeginOverlap
  (params (OtherActor :type Actor%20Object%20Reference))
  (|CallParentFunction OtherActor) ; This node is disabled and will not be called.\nDrag off pins to build functionality.
)

(event EventTick
  (params (DeltaSeconds :type Float%20%28single-precision%29))
  (|CallParentFunction DeltaSeconds) ; This node is disabled and will not be called.\nDrag off pins to build functionality.
)

(event EventOpenDoor
  (Variables|Default|SethasInteracted true)
  (Development|SetHiddeninGame (Variables|Default|Get%20Widget) true false)
  (Utilities|FlowControl|Sequence
    (:then_0
      (bind _rotationpivot (Timeline|OuverturePorte1 Play)
        (:Update
          (Transformation|SetRelativeRotation (Variables|Default|GetPointDoor1) (Math|Rotator|MakeRotator 0.0 0.0 _rotationpivot) false false))))
    (:then_1
      (bind _rotationpivot_2 (Timeline|OuverturePorte2 Play)
        (:Update
          (Transformation|SetRelativeRotation (Variables|Default|GetPointDoor2) (Math|Rotator|MakeRotator 0.0 0.0 _rotationpivot_2) false false))))
    (:then_2
      (Variables|Default|SetisUnlocked true))))

(fn ConstructionScript
  (|CallParentFunction))