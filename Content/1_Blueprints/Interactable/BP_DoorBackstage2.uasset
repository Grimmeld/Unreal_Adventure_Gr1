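; BP_DoorBackstage2 is an interactable backstage door that swings open and records itself as unlocked.
; OpenDoor marks the interaction, hides the widget, starts a timeline that drives the yaw of PointDoor2, and sets IsUnlocked.
; On BeginPlay, an already unlocked door calls SetDoorOpened to appear open without playing the animation.
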(event EventBeginPlay
  (|CallParentFunction)
  (if (Variables|Default|GetisUnlocked)
    (CallFunction|SetDoorOpened -9e+01)))

(event Collision|EventActorBeginOverlap
  (params (OtherActor :type Actor%20Object%20Reference))
  (|CallParentFunction OtherActor) ; This node is disabled and will not be called.\nDrag off pins to build functionality.
)

(event EventTick
  (params (DeltaSeconds :type Float%20%28single-precision%29))
  (|CallParentFunction DeltaSeconds) ; This node is disabled and will not be called.\nDrag off pins to build functionality.
)

(event EventOpenDoor
  (Variables|Default|SethasInteracted true)
  (Development|SetHiddeninGame (Variables|Default|Get%20Widget) true false)
  (Utilities|FlowControl|Sequence
    (:then_0
      (bind _trackporte2 (Timeline|Timeline Play)
        (:Update
          (Transformation|SetRelativeRotation (Variables|Default|GetPointDoor2) (Math|Rotator|MakeRotator 0.0 0.0 _trackporte2) false false))))
    (:then_2
      (Variables|Default|SetisUnlocked true))))

(fn ConstructionScript
  (|CallParentFunction))