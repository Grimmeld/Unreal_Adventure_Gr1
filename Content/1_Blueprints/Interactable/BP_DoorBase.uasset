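; Base interactable door Blueprint that opens freely or with a required inventory item, and can be locked by progression.
; TriggerFront overlaps register it as the character's interactable and toggle the interact prompt, while Tick turns its widget toward the camera.
; UseInteractable consumes the key or logs a refusal, with matching sounds.
; OpenDoor is an empty event, while helper events set the two door pivots' rotations.
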(event OnComponentBeginOverlap(TriggerFront)
  (params (OverlappedComponent :type Primitive%20Component%20Object%20Reference) (OtherActor :type Actor%20Object%20Reference) (OtherComp :type Primitive%20Component%20Object%20Reference) (OtherBodyIndex :type Integer) (bFromSweep :type Boolean) (SweepResult :type Hit%20Result%20Structure%20%28by%20ref%29))
  ;[0.15 0.15 0.15 0.5] Overlap with player
  (bind _asbp_top_down_character (Utilities|Casting|CastToBP_TopDownCharacter OtherActor))
  (CallFunction|InteractionDoor _asbp_top_down_character true false true))

(event OnComponentEndOverlap(TriggerFront)
  (params (OverlappedComponent :type Primitive%20Component%20Object%20Reference) (OtherActor :type Actor%20Object%20Reference) (OtherComp :type Primitive%20Component%20Object%20Reference) (OtherBodyIndex :type Integer))
  ;[0.15 0.15 0.15 0.5] Overlap with player
  (bind _asbp_top_down_character (Utilities|Casting|CastToBP_TopDownCharacter OtherActor))
  (CallFunction|InteractionDoor _asbp_top_down_character false true false))

(event Custom|OpenDoor)

(event Custom|SetDoorOpened
  (params (DoorOuverture :type Float%20%28double-precision%29))
  (Transformation|SetWorldRotation (Variables|Default|GetPointDoor1) (Math|Rotator|MakeRotator 0.0 0.0 (* DoorOuverture -1.0)) false false)
  (Transformation|SetWorldRotation (Variables|Default|GetPointDoor2) (Math|Rotator|MakeRotator 0.0 0.0 DoorOuverture) false false))

(event Custom|LockedByProgression
  (Transformation|SetWorldRotation (Variables|Default|GetPointDoor1) (Math|Rotator|MakeRotator 0.0 0.0 9e+01) false false)
  (Transformation|SetWorldRotation (Variables|Default|GetPointDoor2) (Math|Rotator|MakeRotator 0.0 0.0 9e+01) false false)
  (Variables|Default|SethasBeenLocked true))

(event Custom|InteractionDoor
  (params (Character :type BP%20Top%20Down%20Character%20Object%20Reference) (EnableInteraction :type Boolean) (DisableWidget :type Boolean) (EnableInterForChara :type Boolean))
  (bind _playerref (Variables|Default|GetPlayerRef))
  (if EnableInteraction
    (Default|SetInteractable Character self)
    (else
      (Default|SetInteractable Character)))
  (Variables|Default|SetCanInteract EnableInteraction)
  (Variables|/Game/1_Blueprints/BP_TopDownCharacter.BP_TopDownCharacter_C|SetCanInteractChara _playerref EnableInterForChara)
  (if (Variables|Default|GetisUnlocked)
    (Development|SetHiddeninGame (Variables|/Game/1_Blueprints/BP_TopDownCharacter.BP_TopDownCharacter_C|GetWidget_Interact (Variables|Default|GetPlayerRef)) true false)
    (else
      (Development|SetHiddeninGame (Variables|/Game/1_Blueprints/BP_TopDownCharacter.BP_TopDownCharacter_C|GetWidget_Interact _playerref) DisableWidget false))))

(event EventBeginPlay
  (|CallParentFunction)
  (Utilities|FlowControl|Sequence
    (:then_0
      (bind _asbp_top_down_character (Utilities|Casting|CastToBP_TopDownCharacter (Game|Player|GetPlayerPawn 0)))
      (Variables|Default|SetPlayerRef _asbp_top_down_character)
      (Development|SetHiddeninGame (Variables|Default|Get%20Widget) true false))))

(event EventTick
  (params (DeltaSeconds :type Float%20%28single-precision%29))
  (bind __widget (Variables|Default|Get%20Widget))
  ;[0.15 0.15 0.15 0.5] Move widget with camera
  (if (Variables|Default|GetCanInteract)
    (Transformation|SetWorldRotation __widget (Math|Rotator|FindLookatRotation (Transformation|GetWorldLocation __widget) (Transformation|GetActorLocation (Pawn|GetViewTarget (Variables|/Game/1_Blueprints/BP_TopDownCharacter.BP_TopDownCharacter_C|GetControllerRef (Variables|Default|GetPlayerRef))))) false false)))

(event EventUseInteractable
  (bind _requireitem (Variables|Default|GetRequireItem))
  (bind _playerref (Variables|Default|GetPlayerRef))
  (if (Variables|Default|GethasBeenLocked)
    (Default|AddMessageLog (Variables|/Game/1_Blueprints/BP_TopDownCharacter.BP_TopDownCharacter_C|GetHUDRef (Variables|Default|GetPlayerRef)) (Variables|Log|GetDoorLockedProgLog))
    (Audio|PlaySoundatLocation "/Game/8_Sound/SFX/jp_lockedknob08-42735.jp_lockedknob08-42735" (Transformation|GetActorLocation) "0, 0, 0" 1.0 1.0 0.0 0 0 0 0)
    (elif (not (Variables|Default|GetisUnlocked))
      (if (not (Variables|Default|GethasInteracted))
        (if (== _requireitem "/Game/1_Blueprints/Items/Datas/DA_Item_Empty.DA_Item_Empty")
          (CallFunction|OpenDoor)
          (Audio|PlaySoundatLocation "/Game/8_Sound/SFX/door-opening-454242.door-opening-454242" (Transformation|GetActorLocation) "0, 0, 0" 1.0 1.0 0.0 0 0 0 0)
          (else
            (bind (_found _indexitem) (Default|HasItem _playerref _requireitem))
            (if _found
              (CallFunction|OpenDoor)
              (Default|ConsumeItem (Variables|Default|GetPlayerRef) _indexitem)
              (Audio|PlaySoundatLocation "/Game/8_Sound/SFX/door-opening-454242.door-opening-454242" (Transformation|GetActorLocation) "0, 0, 0" 1.0 1.0 0.0 0 0 0 0)
              (Variables|Default|SetisUnlocked true)
              (else
                (Default|AddMessageLog (Variables|/Game/1_Blueprints/BP_TopDownCharacter.BP_TopDownCharacter_C|GetHUDRef _playerref) (Variables|Log|GetKeyNotFoundLog))
                (Audio|PlaySoundatLocation "/Game/8_Sound/SFX/jp_lockedknob08-42735.jp_lockedknob08-42735" (Transformation|GetActorLocation) "0, 0, 0" 1.0 1.0 0.0 0 0 0 0)))))))))

(fn ConstructionScript
  (|CallParentFunction))