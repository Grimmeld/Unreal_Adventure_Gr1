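; BP_HiddenMessage is an actor in the Mask system that holds one visible message and three hidden, color-named variants (blue, yellow, green).
; On BeginPlay it gathers the four text components into an array and fills them from its text variables.
; ChangeTextDisplay hides every text, then reveals the one whose object name matches the given name.
; Separate events hide all texts or unhide the main message.
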(event Custom|SetHiddenTexts
  (Rendering|Components|TextRender|SetText (Variables|Default|GetHidden1) (Variables|Default|GetHidden1Blue))
  (Rendering|Components|TextRender|SetText (Variables|Default|GetHidden2) (Variables|Default|GetHidden2Yellow))
  (Rendering|Components|TextRender|SetText (Variables|Default|GetHidden3) (Variables|Default|GetHidden3Green))
  (Rendering|Components|TextRender|SetText (Variables|Default|GetMainMessage) (Variables|Default|GetVisibleMessage)))

(event Custom|ShowVisibleMessage
  (Development|SetHiddeninGame (Variables|Default|GetMainMessage) false false))

(event Custom|HideTexts
  (for _array_element (Variables|Default|GetTextsActor)
    (Development|SetHiddeninGame _array_element true false)))

(event Custom|ChangeTextDisplay
  (params (NameText :type String))
  (CallFunction|HideTexts)
  (for _array_element (Variables|Default|GetTextsActor)
    (if (Utilities|Enum|Equal(Enum) (Utilities|GetObjectName _array_element) NameText)
      (Development|SetHiddeninGame _array_element false false))))

(event EventBeginPlay
  (Variables|Default|SetTextsActor (Utilities|Array|MakeArray (Variables|Default|GetHidden1) (Variables|Default|GetHidden2) (Variables|Default|GetHidden3) (Variables|Default|GetMainMessage)))
  (CallFunction|SetHiddenTexts))

(fn ConstructionScript)