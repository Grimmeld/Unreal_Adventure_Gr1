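; Teleport trigger actor that moves the top-down player character to its TeleportPoint, then walks them on to a WalkingPoint.
; Box overlap flags the character as teleporting, disables input, stops movement, relocates it and issues a SimpleMoveToLocation.
; Tick clears the flag and restores input once the player's mesh is within DistanceReset of the WalkingPoint.
; The flag blocks re-triggering mid-teleport; two cube components are destroyed on BeginPlay.
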(event OnComponentBeginOverlap(Box)
  (params (OverlappedComponent :type Primitive%20Component%20Object%20Reference) (OtherActor :type Actor%20Object%20Reference) (OtherComp :type Primitive%20Component%20Object%20Reference) (OtherBodyIndex :type Integer) (bFromSweep :type Boolean) (SweepResult :type Hit%20Result%20Structure%20%28by%20ref%29))
  (bind _teleportpoint (Variables|Default|GetTeleportPoint))
  (bind _asbp_top_down_character (Utilities|Casting|CastToBP_TopDownCharacter OtherActor))
  (if (not (Variables|/Game/1_Blueprints/BP_TopDownCharacter.BP_TopDownCharacter_C|GetIsTeleporting _asbp_top_down_character))
    (Default|SetTeleporting _asbp_top_down_character true)
    (Input|DisableInput (Variables|/Game/1_Blueprints/BP_TopDownCharacter.BP_TopDownCharacter_C|GetControllerRef _asbp_top_down_character) (Variables|/Game/1_Blueprints/BP_TopDownCharacter.BP_TopDownCharacter_C|GetControllerRef _asbp_top_down_character))
    (AI|Navigation|StopMovement (Variables|/Game/1_Blueprints/BP_TopDownCharacter.BP_TopDownCharacter_C|GetControllerRef _asbp_top_down_character))
    (Transformation|SetActorLocationAndRotation _asbp_top_down_character (Transformation|GetWorldLocation _teleportpoint) (Variables|/Script/Engine.SceneComponent|GetRelativeRotation _teleportpoint) false true)
    (bind _output_get (Variables|/Game/1_Blueprints/BP_TopDownController.BP_TopDownController_C|SetCachedDestination (Variables|/Game/1_Blueprints/BP_TopDownCharacter.BP_TopDownCharacter_C|GetControllerRef _asbp_top_down_character) (Transformation|GetWorldLocation (Variables|Default|GetWalkingPoint))))
    (AI|Navigation|SimpleMovetoLocation (Variables|/Game/1_Blueprints/BP_TopDownCharacter.BP_TopDownCharacter_C|GetControllerRef _asbp_top_down_character) _output_get)))

(event EventTick
  (params (DeltaSeconds :type Float%20%28single-precision%29))
  (bind _playerref (Variables|Default|GetPlayerRef))
  (bind _playerref_2 (Variables|Default|GetPlayerRef))
  (bind _controllerref (Variables|/Game/1_Blueprints/BP_TopDownCharacter.BP_TopDownCharacter_C|GetControllerRef _playerref))
  (if (Variables|/Game/1_Blueprints/BP_TopDownCharacter.BP_TopDownCharacter_C|GetIsTeleporting _playerref_2)
    (if (<= (Math|Vector|Distance(Vector) (Transformation|GetWorldLocation (Variables|Default|GetWalkingPoint)) (Transformation|GetWorldLocation (Variables|/Script/Engine.Character|GetMesh _playerref_2))) (Variables|Default|GetDistanceReset))
      (Default|SetTeleporting (Variables|Default|GetPlayerRef) false)
      (Input|EnableInput _controllerref _controllerref))))

(event EventBeginPlay
  (bind _asbp_top_down_character (Utilities|Casting|CastToBP_TopDownCharacter (Game|Player|GetPlayerPawn 0)))
  (Variables|Default|SetPlayerRef _asbp_top_down_character)
  (Components|DestroyComponent (Variables|Default|GetCube))
  (Components|DestroyComponent (Variables|Default|GetCube1)))

(fn ConstructionScript)